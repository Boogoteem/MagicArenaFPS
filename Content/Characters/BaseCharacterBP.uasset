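; Base character Blueprint that handles forward/backward movement and sprinting from pressed and released input actions.
; Each tick eases ForwardSpeed by WalkAcc and feeds it as movement input along control rotation, ignoring pitch when walking or falling.
; Holding Sprint and Forward without Backward triggers a timeline, reversed on stop, that drives max walk speed and issues a mapped FOV console command.
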(event Custom|StartSprinting
  (bind _speedease (Timeline|speedEase Play)
    (:Update
      (Variables|/Script/Engine.CharacterMovementComponent|SetMaxWalkSpeed (Variables|Character|GetCharacterMovement) _speedease)
      (Development|ExecuteConsoleCommand (Utilities|String|Append "fov " (Utilities|String|ToString(Float) (Class|KismetMathLibrary|MapRange _speedease 3e+02 5e+02 95.0 112.0)))))))

(event Custom|StopSprinting
  (bind _speedease (Timeline|speedEase Reverse)
    (:Update
      (Variables|/Script/Engine.CharacterMovementComponent|SetMaxWalkSpeed (Variables|Character|GetCharacterMovement) _speedease)
      (Development|ExecuteConsoleCommand (Utilities|String|Append "fov " (Utilities|String|ToString(Float) (Class|KismetMathLibrary|MapRange _speedease 3e+02 5e+02 95.0 112.0)))))))

(event EventBeginPlay
  (Variables|/Script/Engine.CharacterMovementComponent|SetMaxWalkSpeed (Variables|Character|GetCharacterMovement) 3e+02)
  (Development|ExecuteConsoleCommand "fov 97"))

(event EventTick
  (params (DeltaSeconds :type Float%20%28single-precision%29))
  (CallFunction|UpdateSprinting)
  (CallFunction|UpdateWalkSpeed)
  (CallFunction|AddWalking))

(event Input|ActionEvents|InputActionSprint
  (:Pressed
    (Variables|Default|SetsprintPressed true))
  (:Released
    (Variables|Default|SetsprintPressed false)))

(event Input|ActionEvents|InputActionBackward
  (:Pressed
    (Variables|Default|SetbackwardPressed true))
  (:Released
    (Variables|Default|SetbackwardPressed false)))

(event Input|ActionEvents|InputActionForward
  (:Pressed
    (Variables|Default|SetforwardPressed true))
  (:Released
    (Variables|Default|SetforwardPressed false)))

(fn ConstructionScript)

(fn UpdateWalkSpeed
  (if (Math|Boolean|ORBoolean (and (Variables|Default|GetbackwardPressed) (== -1.0 (Variables|Default|GetforwardSpeed))) (and (== 1.0 (Variables|Default|GetforwardSpeed)) (Variables|Default|GetforwardPressed)) (Math|Boolean|ANDBoolean (== 0.0 (Variables|Default|GetforwardSpeed)) (not (Variables|Default|GetbackwardPressed)) (not (Variables|Default|GetforwardPressed))))
    _
    (elif (Variables|Default|GetforwardPressed)
      (Variables|Default|SetforwardSpeed (+ (Variables|Default|GetforwardSpeed) (Variables|Default|GetwalkAcc)))
      (if (> (Variables|Default|GetforwardSpeed) 1.0) :!label _label
        (Variables|Default|SetforwardSpeed 1.0))
      (else
        (if (Variables|Default|GetbackwardPressed)
          _
          (elif (< (Variables|Default|GetforwardSpeed) 0.0)
            (Variables|Default|SetforwardSpeed (+ (Variables|Default|GetforwardSpeed) (Variables|Default|GetwalkAcc)))
            (goto _label)
            (else
              _)))
        (Variables|Default|SetforwardSpeed (- (Variables|Default|GetforwardSpeed) (Variables|Default|GetwalkAcc)))
        (if (< (Variables|Default|GetforwardSpeed) -1.0)
          (Variables|Default|SetforwardSpeed -1.0)))))
  (return))

(fn AddWalking
  (bind _returnvalue (Pawn|GetController))
  (bind _charactermovement (Variables|Character|GetCharacterMovement))
  (bind _forwardspeed (Variables|Default|GetforwardSpeed))
  (bind _returnvalue_2 (Pawn|GetControlRotation _returnvalue :!class /Script/Engine.Controller))
  (bind (_pitch _yaw _roll) (Class|KismetMathLibrary|BreakRot _returnvalue_2))
  (if (or (AI|Components|NavMovement|IsMovingonGround _charactermovement) (AI|Components|NavMovement|IsFalling _charactermovement))
    (Pawn|Input|AddMovementInput (Math|Rotator|GetRotationXVector (Class|KismetMathLibrary|MakeRot 0.0 _yaw _roll)) _forwardspeed false)
    (else
      (Pawn|Input|AddMovementInput (Math|Rotator|GetRotationXVector (Pawn|GetControlRotation (Pawn|GetController) :!class /Script/Engine.Controller)) _forwardspeed false)))
  (return))

(fn UpdateSprinting
  (Math|Integer|CompareInt (Math|Conversions|ToInteger(Boolean) (Variables|Default|GetisSprinting)) (Math|Conversions|ToInteger(Boolean) (Variables|Default|GetlastIsSprinting))
    (:>
      (Variables|Default|SetlastIsSprinting (Variables|Default|GetisSprinting))
      (CallFunction|StartSprinting))
    (:==
      _)
    (:<
      (Variables|Default|SetlastIsSprinting (Variables|Default|GetisSprinting))
      (CallFunction|StopSprinting)))
  (if (Math|Boolean|ANDBoolean (Variables|Default|GetforwardPressed) (Variables|Default|GetsprintPressed) (not (Variables|Default|GetbackwardPressed)))
    (Variables|Default|SetisSprinting true)
    (else
      (Variables|Default|SetisSprinting false)))
  (return))