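; In-game HUD Blueprint that draws the crosshair and a spell cast indicator around screen center.
; Each DrawHUD scales icon and spell cast sizes to the window through GetScaledGUISize.
; It layers left, center and right crosshair textures in the same rectangle, then draws the SpellCastUI material on top.
; Screen offsets use the unscaled sizes, so elements center exactly only when scaled size equals the original.
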(event EventDrawHUD
  (params (SizeX :type Integer) (SizeY :type Integer))
  (bind _returnvalue (/ SizeY 2))
  (bind _returnvalue_2 (/ SizeX 2))
  (bind _renderediconsize (Variables|Default|GetrenderedIconSize))
  (bind _renderedspellcastsize (Variables|Default|GetrenderedSpellCastSize))
  (bind _returnvalue_3 (/ _renderedspellcastsize 2))
  (bind _returnvalue_4 (/ _renderediconsize 2))
  (bind _returnvalue_5 (- _returnvalue_2 _returnvalue_4))
  (bind _returnvalue_6 (- _returnvalue _returnvalue_4))
  (bind _returnvalue_7 (Math|Conversions|ToFloat(Integer) _returnvalue_6))
  (bind _returnvalue_8 (Math|Conversions|ToFloat(Integer) _returnvalue_5))
  (bind (_scaledw _scaledh) (CallFunction|GetScaledGUISize SizeX SizeY _renderedspellcastsize _renderedspellcastsize))
  (bind (_scaledw_2 _scaledh_2) (CallFunction|GetScaledGUISize SizeX SizeY _renderediconsize _renderediconsize))
  (Canvas|DrawTexture "/Game/HUDs/Textures/crosshair_left.crosshair_left" _returnvalue_8 _returnvalue_7 _scaledw_2 _scaledh_2 0.0 0.0 1.0 1.0 "(R=1.000000,G=1.000000,B=1.000000,A=1.000000)")
  (Canvas|DrawTexture "/Game/HUDs/Textures/crosshair_center.crosshair_center" _returnvalue_8 _returnvalue_7 _scaledw_2 _scaledh_2 0.0 0.0 1.0 1.0 "(R=1.000000,G=1.000000,B=1.000000,A=1.000000)")
  (Canvas|DrawTexture "/Game/HUDs/Textures/crosshair_right.crosshair_right" _returnvalue_8 _returnvalue_7 _scaledw_2 _scaledh_2 0.0 0.0 1.0 1.0 "(R=1.000000,G=1.000000,B=1.000000,A=1.000000)")
  (Class|HUD|DrawMaterialSimple "/Game/HUDs/Widgets/DynamicCircleMask/MICs/SpellCastUI.SpellCastUI" (Math|Conversions|ToFloat(Integer) (- _returnvalue_2 _returnvalue_3)) (Math|Conversions|ToFloat(Integer) (- _returnvalue _returnvalue_3)) _scaledw _scaledh 1.0 false))

(fn ConstructionScript)